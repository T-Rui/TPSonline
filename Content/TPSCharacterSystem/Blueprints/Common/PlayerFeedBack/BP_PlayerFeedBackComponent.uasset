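; BP_PlayerFeedBackComponent manages player feedback in the form of camera shakes on the first player's camera manager.
; Single and looped plays both stop all active shakes first, so each new request replaces the last.
; Looping replays the stored shake class on a repeating timer at the supplied interval.
; A targeted stop clears that timer and ends the current shake immediately, but only when its class matches the requested one.
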(event `PlaySingleCamShake`
  (params (`Camera Shake Type` :type "CameraShake Class Reference"))
  ;[1 1 1] PlaySingleCamShake
  ;;[1 1 1] Stop All Cam Shakes
  (`self.StopAllCameraShakes`)
  ;;[1 1 1] Initialize Values
  (set `self.Camera Shake Type` `Camera Shake Type`)
  (bind _returnvalue (`PlayerCameraManager.PlayCameraShake` :`self` (`GameplayStatics.GetPlayerCameraManager` 0) :`ShakeClass` (`self.Camera Shake Type`)))
  (set `self.CurrentCamShake` _returnvalue))

(event `PlayLoopCameraShake`
  (params (`Camera Shake Type` :type "CameraShake Class Reference") (`Loop Time` :type "Float (double-precision)"))
  ;[1 1 1] Start loop Cam Shake
  ;;[1 1 1] Stop All Cam Shakes
  (`self.StopAllCameraShakes`)
  ;;[1 1 1] Initialize Values
  (set `self.Camera Shake Type` `Camera Shake Type`)
  (set `self.Loop Type` `Loop Time`)
  ;;[1 1 1] Create Shakes
  (`self.CreateCameraShake`)
  (`KismetSystemLibrary.K2_SetTimer` null "CreateCameraShake" (`self.Loop Type`) true))

(event `StopCameraShake`
  (params (`Camera Shake Type` :type "CameraShake Class Reference"))
  ;[1 1 1] Stop Cam Shake
  (if (== `Camera Shake Type` (`GameplayStatics.GetObjectClass` (`self.CurrentCamShake`)))
    (`KismetSystemLibrary.K2_ClearTimer` null "CreateCameraShake")
    (`PlayerCameraManager.StopCameraShake` (`GameplayStatics.GetPlayerCameraManager` 0) (`self.CurrentCamShake`) true)))

(event `CreateCameraShake`
  ;[1 1 1] CREATE CAMERA SHAKE
  (bind _returnvalue (`PlayerCameraManager.PlayCameraShake` :`self` (`GameplayStatics.GetPlayerCameraManager` 0) :`ShakeClass` (`self.Camera Shake Type`)))
  (set `self.CurrentCamShake` _returnvalue))

(event `StopAllCameraShakes`
  ;[1 1 1] StopAllCameraShakes
  (`KismetSystemLibrary.K2_ClearTimer` null "CreateCameraShake")
  (`PlayerCameraManager.StopAllCameraShakes` (`GameplayStatics.GetPlayerCameraManager` 0) true))