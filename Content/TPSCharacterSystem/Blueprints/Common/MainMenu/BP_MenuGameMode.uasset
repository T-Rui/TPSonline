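; Main menu game mode that tracks players in the multiplayer lobby and starts the match.
; On the authority, login and logout update a player controller list, then after a short delay push the new count to every menu controller.
; GameStart calls StartGame on each listed controller, then issues a servertravel console command targeting the playground level.
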(event `GameStart`
  ;[1 1 1] START GAME
  (for _array_element (`self.PlayersList`)
    (bind _asbp_menu_player_controller (cast `/Game/TPSCharacterSystem/Blueprints/Common/MainMenu/BP_MenuPlayerController` _array_element))
    (`/Game/TPSCharacterSystem/Blueprints/Common/MainMenu/BP_MenuPlayerController.StartGame` _asbp_menu_player_controller))
  (`KismetSystemLibrary.ExecuteConsoleCommand` "servertravel/game/TPSCharacterSystem/Levels/playground" (`GameplayStatics.GetPlayerController` 0)))

(event `self.K2_PostLogin`
  (params (NewPlayer :type "PlayerController Object Reference"))
  ;[1 1 1] UPDATE PLR COUNT
  ;;[1 1 1] On Joined
  (`/Engine/EditorBlueprintResources/ActorMacros.Switch Has Authority`
    (:`Authority`
      (`KismetArrayLibrary.Array_Add` (`self.PlayersList`) NewPlayer)
      ;;[1 1 1] Update current Plr Count
      (`KismetSystemLibrary.Delay` 0.2 :!label _label)
      (for _array_element (`self.PlayersList`)
        (bind _asbp_menu_player_controller (cast `/Game/TPSCharacterSystem/Blueprints/Common/MainMenu/BP_MenuPlayerController` _array_element))
        (`/Game/TPSCharacterSystem/Blueprints/Common/MainMenu/BP_MenuPlayerController.UpdatePlayersCounInLobby` _asbp_menu_player_controller (`KismetArrayLibrary.Array_Length` (`self.PlayersList`)))))))

(event `self.K2_OnLogout`
  (params (ExitingController :type "Controller Object Reference"))
  ;[1 1 1] UPDATE PLR COUNT
  ;;[1 1 1] On Leave
  (`/Engine/EditorBlueprintResources/ActorMacros.Switch Has Authority`
    (:`Authority`
      (bind _asbp_menu_player_controller (cast `/Game/TPSCharacterSystem/Blueprints/Common/MainMenu/BP_MenuPlayerController` ExitingController))
      (`KismetArrayLibrary.Array_RemoveItem` (`self.PlayersList`) _asbp_menu_player_controller)
      (goto _label))))

(fn `UserConstructionScript`)