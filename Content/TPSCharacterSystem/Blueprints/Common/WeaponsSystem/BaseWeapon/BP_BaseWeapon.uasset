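; Base weapon Blueprint for a third-person shooter character system, handling ammo setup and firing effects.
; BeginPlay fills clip and reserve ammo from WeaponSetting and converts rounds per minute into a delay between shots.
; PlaySFXSound relays through ToServer and ToAll events to play muzzle sound and flash, then terminates them after a short delay.
; A DoOnce blocks repeat effects until termination destroys the emitter and resets it; separate trail logic is disconnected.
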(event `self.ReceiveBeginPlay`
  (bind (_firerate _clipsize _ammosize) (break `/Game/TPSCharacterSystem/Blueprints/Common/WeaponsSystem/STR_WeaponsSettings` (`self.WeaponSetting`)))
  ;[1 1 1] Event Begin
  (set `self.CurrentAmmoInClip` _clipsize)
  (set `self.CurrentAmmoPull` _ammosize)
  (set `self.Shots Delay` (/ 1.0 (/ (`KismetMathLibrary.Conv_IntToDouble` _firerate) 60.0))))

(event `PlaySFXSound`
  ;[1 1 1] Comment
  (`self.PlayToServerWeaponSFX`)
  (`KismetSystemLibrary.Delay` 0.16)
  (`self.TerminateToServerWeaponSFX`))

(event `PlayToServerWeaponSFX`
  ;[1 1 1] PlayToServerWeaponSFX
  (`self.PlayToAllWeaponSFX`))

(event `TerminateToServerWeaponSFX`
  ;[1 1 1] TerminateToServerWeaponSFX
  (`self.TerminateToAllWeaponSFX`))

(event `TerminateToAllWeaponSFX`
  (bind _skeletalmesh (`self.SkeletalMesh`))
  (bind _returnvalue (`SceneComponent.GetSocketLocation` _skeletalmesh "Muzzle"))
  ;[1 1 1] PlayToAllWeaponSFX // TerminateToAllWeaponSFX
  (`|ExecutionSequence`
    (:`then_0`
      (`/Engine/EditorBlueprintResources/StandardMacros.IsValid` (stale `PlayToAllWeaponSFX` _returnvalue_2)
        (:`Is Valid`
          (`ActorComponent.K2_DestroyComponent` (stale `PlayToAllWeaponSFX` _returnvalue_2)))))
    (:`then_1`
      (goto _label :!via `Reset`))))

(event `PlayToAllWeaponSFX`
  (bind _skeletalmesh (`self.SkeletalMesh`))
  (bind _returnvalue (`SceneComponent.GetSocketLocation` _skeletalmesh "Muzzle"))
  ;[1 1 1] PlayToAllWeaponSFX // TerminateToAllWeaponSFX
  (`/Engine/EditorBlueprintResources/StandardMacros.DoOnce` false :!label _label
    (:`Completed`
      (`GameplayStatics.PlaySoundAtLocation` "/Game/TPSCharacterSystem/Demo/Sound/Wave/Weapons/AssaultRifle_Shot01_Stereo.AssaultRifle_Shot01_Stereo" _returnvalue (struct) 1.0 1.0 0.0 null null null)
      (bind _returnvalue_2 (`GameplayStatics.SpawnEmitterAttached` "/Game/TPSCharacterSystem/Demo/Effects/ParticleSystems/P_AssaultRifle_MF.P_AssaultRifle_MF" _skeletalmesh "Muzzle" _returnvalue (`SceneComponent.GetSocketRotation` _skeletalmesh "Muzzle") (1.0 1.0 1.0) "KeepWorldPosition" false)))))

(fn `UserConstructionScript`)