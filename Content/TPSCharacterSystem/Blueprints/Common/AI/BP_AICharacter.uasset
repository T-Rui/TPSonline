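; AI character Blueprint for the TPS character system that sets up an armed AI through its InitializeAI event.
; It spawns primary and secondary weapons, initializes the current one via a server call, then attaches both to the mesh's GunSocket.
; After a short delay for spawning, it initializes the weapon system with damageable actor classes and an arrow for shooting.
; BeginPlay, Tick and construction only call the parent.
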(event `self.ReceiveBeginPlay`
  (`parent.ReceiveBeginPlay`))

(event `InitializeAI`
  (params (ActorsClassForTakeDamage :type "Array of Object Class Reference (by ref)") (`Primary Weapon` :type "Actor Class Reference") (`Secondary Weapon` :type "Actor Class Reference"))
  (`|ExecutionSequence`
    (:`then_0`
      ;[1 1 1] COMMON START EVENTS. USING IN ALL VERSION OF THE PLATFORM
      ;;[0.5 0 0.00927] SpawnShowHideWeapons
      (`self.SpawnShowHideWeapons` `Primary Weapon` `Secondary Weapon` (`SceneComponent.GetRelativeTransform` (`self.Mesh`)))
      ;;[0.5 0 0.00927] InitializeCurrentWeaponInCharacter
      (`self.ServerInitializeCurrentWeaponInCharacter`)
      ;[1 1 1] CHILD START EVENTS. SPECIFIC FOR TPS CS
      ;;[1 1 1] [child event]
      (`self.TPSAttachWeapons`))
    (:`then_1`
      ;[1 1 1] COMMON START EVENTS. USING IN ALL VERSION OF THE PLATFORM
      ;;[1 1 1] [wait spawn weapons]
      (`KismetSystemLibrary.Delay` 0.2)
      ;;[0.5 0 0.00927] CommonInitializeWeaponSystem
      (`self.CommonInitializeWeaponSystem` null self (`self.ShootingArrow`) true false ActorsClassForTakeDamage)
      ;;[0.5 0 0.00927] InitializeWeaponInWeaponSystem
      (`self.InitializeWeaponInWeaponSystem`))))

(event `self.ReceiveTick`
  (params (DeltaSeconds :type "Float (single-precision)"))
  (`parent.ReceiveTick` DeltaSeconds))

(event `TPSAttachWeapons`
  ;[1 1 1] CHILD CLASS SPECIFIC INITIALIZE EVENTS
  ;;[1 1 1] TPS ATTACH WEAPONS
  (`|ExecutionSequence`
    (:`then_0`
      (`/Engine/EditorBlueprintResources/StandardMacros.IsValid` (`self.PrimaryWeapon`)
        (:`Is Valid`
          (`self.K2_AttachToComponent` (`self.PrimaryWeapon`) (`self.Mesh`) "GunSocket" "SnapToTarget" "KeepRelative" "KeepRelative" true))))
    (:`then_1`
      (`/Engine/EditorBlueprintResources/StandardMacros.IsValid` (`self.SecondaryWeapon`)
        (:`Is Valid`
          (`self.K2_AttachToComponent` (`self.SecondaryWeapon`) (`self.Mesh`) "GunSocket" "SnapToTarget" "KeepRelative" "KeepRelative" true))))))

(fn `UserConstructionScript`
  (`parent.UserConstructionScript`))