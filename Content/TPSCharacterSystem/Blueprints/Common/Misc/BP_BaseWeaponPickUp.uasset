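; Base weapon pickup actor that displays a spawned weapon and lets characters swap their weapon with it.
; On BeginPlay it spawns the weapon class slightly raised and rolled onto its side, then caches its ammo.
; Sphere overlaps, gated by a CanUse flag, toggle the pickup permission on BP_CommonCharacter.
; A multicast-named event handles swaps by respawning the given weapon class and restoring the passed-in clip and reserve ammo.
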(event `self.ReceiveBeginPlay`
  ;[1 1 1] START SPAWN WEAPON PICK UP & INITIALIZE
  (`self.InitializePickUP`)
  ;;[1 1 1] Ini def ammo settings
  (bind _asbp_base_weapon (cast `/Game/TPSCharacterSystem/Blueprints/Common/WeaponsSystem/BaseWeapon/BP_BaseWeapon` (`self.WeaponPickUp`)))
  (set `self.WeaponCurrentAmmoInClip` (`/Game/TPSCharacterSystem/Blueprints/Common/WeaponsSystem/BaseWeapon/BP_BaseWeapon.CurrentAmmoInClip` _asbp_base_weapon))
  (set `self.WeaponCurrentAmmoPull` (`/Game/TPSCharacterSystem/Blueprints/Common/WeaponsSystem/BaseWeapon/BP_BaseWeapon.CurrentAmmoPull` _asbp_base_weapon)))

(event `InitializePickUP`
  ;[1 1 1] SPAWN WEAPON
  (bind _returnvalue (`|SpawnActorFromClass` (`self.WeaponItemClass`) (`KismetMathLibrary.MakeTransform` (`KismetMathLibrary.MakeVector` (.x (.location (`SceneComponent.GetRelativeTransform` (`self.DefaultSceneRoot`)))) (.y (.location (`SceneComponent.GetRelativeTransform` (`self.DefaultSceneRoot`)))) (+ (.z (.location (`SceneComponent.GetRelativeTransform` (`self.DefaultSceneRoot`)))) 10.0)) (`KismetMathLibrary.MakeRotator` (+ (.roll (.rotation (`SceneComponent.GetRelativeTransform` (`self.DefaultSceneRoot`)))) 90.0) (.pitch (.rotation (`SceneComponent.GetRelativeTransform` (`self.DefaultSceneRoot`)))) (.yaw (.rotation (`SceneComponent.GetRelativeTransform` (`self.DefaultSceneRoot`))))) (.scale (`SceneComponent.GetRelativeTransform` (`self.DefaultSceneRoot`)))) "AlwaysSpawn" "OverrideRootScale" null null))
  (set `self.WeaponPickUp` _returnvalue))

(event `self.Sphere.OnComponentBeginOverlap`
  (params (OverlappedComponent :type "PrimitiveComponent Object Reference") (OtherActor :type "Actor Object Reference") (OtherComp :type "PrimitiveComponent Object Reference") (OtherBodyIndex :type Integer) (bFromSweep :type Boolean) (SweepResult :type "HitResult Structure (by ref)"))
  ;[1 1 1] OVERLAP LOGIC
  (if (`self.CanUse?`)
    (set `self.CanUse?` false)
    (bind _asbp_common_character (cast `/Game/TPSCharacterSystem/Blueprints/Common/BP_CommonCharacter` OtherActor))
    (`/Game/TPSCharacterSystem/Blueprints/Common/BP_CommonCharacter.SetCanPickUpItemClient` _asbp_common_character true)))

(event `self.Sphere.OnComponentEndOverlap`
  (params (OverlappedComponent :type "PrimitiveComponent Object Reference") (OtherActor :type "Actor Object Reference") (OtherComp :type "PrimitiveComponent Object Reference") (OtherBodyIndex :type Integer))
  ;[1 1 1] OVERLAP LOGIC
  (set `self.CanUse?` true)
  (bind _asbp_common_character (cast `/Game/TPSCharacterSystem/Blueprints/Common/BP_CommonCharacter` OtherActor))
  (`/Game/TPSCharacterSystem/Blueprints/Common/BP_CommonCharacter.SetCanPickUpItemClient` _asbp_common_character false))

(event `MultiCastChangePickUpItem`
  (params (CurrentAmmoPull :type Integer) (CurrentAmmoInClip :type Integer) (`Weapon Class` :type "/Game/TPSCharacterSystem/Blueprints/Common/WeaponsSystem/BaseWeapon/BP_BaseWeapon Class Reference"))
  ;[1 1 1] WEAPON FROM THIS PICK UP CHANDED TO PLR WEAPON
  ;;[1 1 1] INIT VALUES
  (set `self.WeaponCurrentAmmoPull` CurrentAmmoPull)
  (set `self.WeaponCurrentAmmoInClip` CurrentAmmoInClip)
  (set `self.WeaponItemClass` `Weapon Class`)
  ;;[1 1 1] DESTROY OLD AND SPAWN NEW
  (`self.K2_DestroyActor` (`self.WeaponPickUp`))
  (`self.InitializePickUP`)
  ;;[1 1 1] SET AMMO VALUES FROM PLR WEAPON
  (bind _asbp_base_weapon (cast `/Game/TPSCharacterSystem/Blueprints/Common/WeaponsSystem/BaseWeapon/BP_BaseWeapon` (`self.WeaponPickUp`)))
  (set `/Game/TPSCharacterSystem/Blueprints/Common/WeaponsSystem/BaseWeapon/BP_BaseWeapon.CurrentAmmoInClip` (`self.WeaponCurrentAmmoInClip`) _asbp_base_weapon)
  (set `/Game/TPSCharacterSystem/Blueprints/Common/WeaponsSystem/BaseWeapon/BP_BaseWeapon.CurrentAmmoPull` (`self.WeaponCurrentAmmoPull`) _asbp_base_weapon))

(fn `UserConstructionScript`)