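; Weapon range target dummy that shows damage taken on a text render, then "dies" and resets to full health.
; AnyDamage feeds a server-named update that uses a short Delay to sum near-simultaneous hits before subtracting health and passing the total to a multicast-named text update.
; At zero health it switches body and head collision from Pawn to Vehicle and blinks for about five seconds, then restores health, collision and blank text.
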(event `self.ReceiveBeginPlay`
  ;[1 1 1] EVENT BEGIN PLAY
  (set `self.CurrentHealth` (`self.MaxHealth`))
  (`TextRenderComponent.K2_SetText` (`self.TextRender`) (`self.EmptyText`)))

(event `self.ReceiveAnyDamage`
  (params (Damage :type "Float (single-precision)") (DamageType :type "DamageType Object Reference") (InstigatedBy :type "Controller Object Reference") (DamageCauser :type "Actor Object Reference"))
  ;[1 1 1] EVENT ANY DAMAGE
  (`self.UpdateDollsHealthServer` Damage))

(event `UpdateDollsHealthServer`
  (params (Damage :type "Float (double-precision)"))
  (bind _returnvalue (- (`self.CurrentHealth`) (`self.TakedDamage`)))
  ;[1 1 1] UPDATE HEALTH - SERVER PART
  (set `self.TakedDamage` (+ (`self.TakedDamage`) Damage))
  (`KismetSystemLibrary.Delay` 0.05)
  (if (<= _returnvalue 0.0)
    (set `self.CurrentHealth` 0.0)
    (set `self.Dead?` true)
    (`self.DollRespawn` (`self.TakedDamage`))
    (`KismetSystemLibrary.Delay` 5.1)
    (set `self.TakedDamage` 0.0)
    (set `self.CurrentHealth` (`self.MaxHealth`))
    (`self.DollReHeath`)
    (set `self.Dead?` false)
    (else
      (set `self.CurrentHealth` _returnvalue)
      (`self.UpdateDollsHealthMultiCast` (`self.TakedDamage`))
      (set `self.TakedDamage` 0.0))))

(event `DollRespawn`
  (params (Damage :type "Float (double-precision)"))
  ;[1 1 1] DOLL DEAD FEEDBACK
  (`TextRenderComponent.K2_SetText` (`self.TextRender`) (`KismetTextLibrary.Conv_DoubleToText` Damage "HalfToEven"))
  (`PrimitiveComponent.SetCollisionObjectType` (`self.Main`) "ECC_Vehicle")
  (`PrimitiveComponent.SetCollisionObjectType` (`self.Head`) "ECC_Vehicle")
  (`self.ToggleVisibl`)
  (`KismetSystemLibrary.Delay` 1.0)
  (`self.ToggleVisibl`)
  (`KismetSystemLibrary.Delay` 1.0)
  (`self.ToggleVisibl`)
  (`KismetSystemLibrary.Delay` 1.0)
  (`self.ToggleVisibl`)
  (`KismetSystemLibrary.Delay` 1.0)
  (`self.ToggleVisibl`)
  (`KismetSystemLibrary.Delay` 1.0)
  (`self.ToggleVisibl`))

(event `DollReHeath`
  ;[1 1 1] DOLL RESPAWN
  (`TextRenderComponent.K2_SetText` (`self.TextRender`) (`self.EmptyText`))
  (`PrimitiveComponent.SetCollisionObjectType` (`self.Main`) "ECC_Pawn")
  (`PrimitiveComponent.SetCollisionObjectType` (`self.Head`) "ECC_Pawn"))

(event `UpdateDollsHealthMultiCast`
  (params (Damage :type "Float (double-precision)"))
  ;[1 1 1] SET DAMAGE TEXT
  (`TextRenderComponent.K2_SetText` (`self.TextRender`) (`KismetTextLibrary.Conv_DoubleToText` Damage "HalfToEven")))

(fn `ToggleVisibl`
  (locals (ReHelingText :type Text :default "NSLOCTEXT(\"\", \"554A405B447DE5F4A63679B3B69DD82B\", \"Target Killed\")"))
  (`SceneComponent.ToggleVisibility` (`self.Main`) false)
  (`SceneComponent.ToggleVisibility` (`self.Head`) false)
  (`SceneComponent.ToggleVisibility` (`self.TextRender`) false))

(fn `UserConstructionScript`)