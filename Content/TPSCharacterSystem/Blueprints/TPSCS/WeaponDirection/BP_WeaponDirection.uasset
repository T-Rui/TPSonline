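; Weapon direction system for a third-person character, computing aim-offset yaw and pitch and the weapon arrow's rotation.
; A camera trace finds the target, then triangle trigonometry from spring arm and muzzle arrow points yields both angle sets, supporting camera mirroring.
; Aim-offset yaw eases through a timer-driven curve, while pitch snaps because its interpolation is unwired.
; Recoil accumulates and recovers separately but is not passed into the final rotation calculation.
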(event `InitializeWeaponDirectionSystem`
  (params (Character :type "/Game/TPSCharacterSystem/Blueprints/TPSCS/BP_TPSCharacter Object Reference"))
  ;[1 1 1] INITIALIZE WEAPON DIRECTION SYSTEM
  (set `self.Character` Character))

(event `CalculationWeaponDirection`
  (params (`CameraMirror?` :type Boolean) (`Collision?` :type Boolean) (`In Minizoom?` :type Boolean) (`Weapon Main Arrow World Loc` :type "Vector Structure") (`Camera World Location` :type "Vector Structure") (`Camera World Rotation` :type "Rotator Structure") (`Spring Arm World Location` :type "Vector Structure") (`Spring Arm Socet Offset` :type "Vector Structure") (`Character Actor Rotation` :type "Rotator Structure"))
  ;[1 1 1] CALCULATION WEAPON DIRECTION / AIM OFF SET
  ;;[1 1 1] Initialize Character States
  (set `self.CameraMirror` `CameraMirror?`)
  (set `self.Collision` `Collision?`)
  (set `self.In Minizoom` `In Minizoom?`)
  (set `self.Wpn Main Arrow World Loc` `Weapon Main Arrow World Loc`)
  (set `self.Camera World Location` `Camera World Location`)
  (set `self.Camera World Rotation` `Camera World Rotation`)
  (set `self.Spring Arm World Location` `Spring Arm World Location`)
  (set `self.Spring Arm Socet Offset` `Spring Arm Socet Offset`)
  (set `self.Character Actor Rotation` `Character Actor Rotation`)
  ;;[1 1 1] Create Weapon Targer from Trace
  (bind _weapontargetlocation (`self.CreateWeaponTargetTrace` (`self.Collision`)))
  (set `self.WeaponTargetLocation` _weapontargetlocation)
  ;;[1 1 1] Aim Off Set PRE Calculation
  (bind (_point_a _point_b _point_c _point_e) (`self.AimOffSetPointsCalculation` (`self.WeaponTargetLocation`)))
  (set `self.Additianal Point B` _point_b)
  (bind (_pre_aim_off_set_yaw _pre_aim_off_set_pitch) (`self.AimOffSetCalculation` _point_a _point_b _point_c _point_e (`self.CameraMirror`)))
  (set `self.Pre Aim Off Set Yaw` _pre_aim_off_set_yaw)
  (set `self.Pre Aim Off Set Pitch` _pre_aim_off_set_pitch)
  ;;[1 1 1] Aim Off Set Yaw & Pitch Smooth Logic
  (if (`self.OnSpawn?`)
    (set `self.Aim Off Set Yaw` (`self.Pre Aim Off Set Yaw`))
    (set `self.Aim Off Set Pitch` (`self.Pre Aim Off Set Pitch`))
    (set `self.OnSpawn?` false))
  (if (`KismetMathLibrary.NearlyEqual_FloatFloat` (`self.Pre Aim Off Set Yaw`) (`self.Aim Off Set Yaw`) 1.5)
    (set `self.Aim Off Set Yaw` (`self.Pre Aim Off Set Yaw`))
    (else
      (`self.StartInterpolationAimOffSetYaw`)))
  (if (`KismetMathLibrary.NearlyEqual_FloatFloat` (`self.Pre Aim Off Set Pitch`) (`self.Aim Off Set Pitch`) 1.5)
    _
    (else
      _))
  (set `self.Aim Off Set Pitch` (`self.Pre Aim Off Set Pitch`))
  ;;[1 1 1] Weapon Direction Calculation  & Recoil Impact
  (bind (_point_a_2 _point_b_2 _point_c_2 _point_e_2) (`self.WeaponDirectionPointCalculation` (`self.WeaponTargetLocation`) (`self.Additianal Point B`) (`self.CameraMirror`) (`self.Wpn Main Arrow World Loc`)))
  (bind (_pre_weapon_yaw _pre_weapon_pitch) (`self.WeaponDirectionPreCalculation` _point_a_2 _point_b_2 _point_c_2 _point_e_2))
  (bind _weapon_direction (`self.WeaponDirectionFinalCalculation` _pre_weapon_yaw _pre_weapon_pitch _point_e_2 _point_c_2 (`self.Pre Aim Off Set Yaw`) (`self.Pre Aim Off Set Pitch`)))
  (set `self.Main Arrow Rotation` _weapon_direction))

(event `StartInterpolationAimOffSetYaw`
  ;[1 1 1] AIM OFF SET YAW & PITCH INTERPOLATION (SMOOTH)
  ;;[1 1 1] Start & Stop Interpolation Aim Off Set Yaw
  (`/Engine/EditorBlueprintResources/StandardMacros.DoOnce` false :!label _label
    (:`Completed`
      (`self.StepInterpolationAimOffSetYaw`)
      (`KismetSystemLibrary.K2_SetTimer` null "StepInterpolationAimOffSetYaw" (`self.Interpolation Step Time`) true))))

(event `UpdateRecoilImpact`
  (params (`In Shooting?` :type Boolean) (VerDeltaRecoil :type "Float (double-precision)") (HorDeltaRecoil :type "Float (double-precision)") (RecDeltaRecoilVer :type "Float (double-precision)") (RecDeltaRecoilHor :type "Float (double-precision)"))
  (bind _recdeltarecoilhor (`self.RecDeltaRecoilHor`))
  ;[1 1 1] UPDATE RECOIL IMPACT ON WEAPON DIRECTION
  ;;[1 1 1] Initialize Character States
  (set `self.In Shooting?` `In Shooting?`)
  (set `self.VerDeltaRecoil` VerDeltaRecoil)
  (set `self.HorDeltaRecoil` HorDeltaRecoil)
  (set `self.RecDeltaRecoilVer` RecDeltaRecoilVer)
  (set `self.RecDeltaRecoilHor` RecDeltaRecoilHor)
  (if (`self.In Shooting?`)
    ;;[1 1 1] In Shooting
    (set `self.Vertical Rec Impact` (+ (`self.Vertical Rec Impact`) (`self.VerDeltaRecoil`)))
    (set `self.Horizontal Rec Impact` (+ (`self.Horizontal Rec Impact`) (`self.HorDeltaRecoil`)))
    (else
      (`|ExecutionSequence`
        (:`then_0`
          ;;[1 1 1] In Recover Ver
          (if (< (`self.Vertical Rec Impact`) 0.1)
            (set `self.Vertical Rec Impact` 0.0)
            (else
              (set `self.Vertical Rec Impact` (- (`self.Vertical Rec Impact`) (`self.RecDeltaRecoilVer`))))))
        (:`then_1`
          ;;[1 1 1] In recover Hor
          (if (< (`self.Horizontal Rec Impact`) 0.05)
            (set `self.Horizontal Rec Impact` 0.0)
            (elif (< _recdeltarecoilhor 0.0)
              (set `self.Horizontal Rec Impact` (+ (`self.Horizontal Rec Impact`) _recdeltarecoilhor))
              (else
                (set `self.Horizontal Rec Impact` (- (`self.Horizontal Rec Impact`) _recdeltarecoilhor))))))))))

(event `StopInterpolationAimOffSetYaw`
  ;[1 1 1] AIM OFF SET YAW & PITCH INTERPOLATION (SMOOTH)
  ;;[1 1 1] Start & Stop Interpolation Aim Off Set Yaw
  (set `self.Interpolation Time Aim Off Set Yaw` 0.0)
  (`KismetSystemLibrary.K2_ClearTimer` null "StepInterpolationAimOffSetYaw")
  (goto _label :!via `Reset`))

(event `StepInterpolationAimOffSetYaw`
  ;[1 1 1] AIM OFF SET YAW & PITCH INTERPOLATION (SMOOTH)
  ;;[1 1 1] Step Interpolation Aim Off Set Yaw
  (`/Engine/EditorBlueprintResources/StandardMacros.IsValid` (`self.Interpolation Curve`)
    (:`Is Valid`
      (if (`KismetMathLibrary.NearlyEqual_FloatFloat` (`self.Pre Aim Off Set Yaw`) (`self.Aim Off Set Yaw`) 1.0)
        (`self.StopInterpolationAimOffSetYaw`)
        (else
          (set `self.Interpolation Time Aim Off Set Yaw` (+ (`self.Interpolation Time Aim Off Set Yaw`) (`self.Interpolation Step Time`)))
          (set `self.Aim Off Set Yaw` (`|EaseFunction` "Linear" (`CurveFloat.GetFloatValue` (`self.Interpolation Curve`) (`self.Interpolation Time Aim Off Set Yaw`)) (`self.Aim Off Set Yaw`) (`self.Pre Aim Off Set Yaw`))))))))

(event `StartInterpolationAimOffSetPitch`
  ;[1 1 1] AIM OFF SET YAW & PITCH INTERPOLATION (SMOOTH)
  ;;[1 1 1] Start & Stop Interpolation Aim Off Set Pitch
  (`/Engine/EditorBlueprintResources/StandardMacros.DoOnce` false :!label _label_2
    (:`Completed`
      (`self.StepInterpolationAimOffSetPitch`)
      (`KismetSystemLibrary.K2_SetTimer` null "StepInterpolationAimOffSetPitch" (`self.Interpolation Step Time`) true))))

(event `StopInterpolationAimOffSetPitch`
  ;[1 1 1] AIM OFF SET YAW & PITCH INTERPOLATION (SMOOTH)
  ;;[1 1 1] Start & Stop Interpolation Aim Off Set Pitch
  (set `self.Interpolation Time Aim Off Set Pitch` 0.0)
  (`KismetSystemLibrary.K2_ClearTimer` null "StepInterpolationAimOffSetPitch")
  (goto _label_2 :!via `Reset`))

(event `StepInterpolationAimOffSetPitch`
  ;[1 1 1] AIM OFF SET YAW & PITCH INTERPOLATION (SMOOTH)
  ;;[1 1 1] Step Interpolation Aim Off Set Pitch
  (`/Engine/EditorBlueprintResources/StandardMacros.IsValid` (`self.Interpolation Curve`)
    (:`Is Valid`
      (if (`KismetMathLibrary.NearlyEqual_FloatFloat` (`self.Pre Aim Off Set Pitch`) (`self.Aim Off Set Pitch`) 1.0)
        (`self.StopInterpolationAimOffSetPitch`)
        (else
          (set `self.Interpolation Time Aim Off Set Pitch` (+ (`self.Interpolation Time Aim Off Set Pitch`) (`self.Interpolation Step Time`)))
          (set `self.Aim Off Set Pitch` (`|EaseFunction` "Linear" (`CurveFloat.GetFloatValue` (`self.Interpolation Curve`) (`self.Interpolation Time Aim Off Set Pitch`)) (`self.Aim Off Set Pitch`) (`self.Pre Aim Off Set Pitch`))))))))

(fn `AimOffSetCalculation`
  (params (`Point A` :type "Vector Structure") (`Point B` :type "Vector Structure") (`Point C` :type "Vector Structure") (`Point E` :type "Vector Structure") (`CameraMirror?` :type Boolean))
  (returns (`Pre Aim Off Set Yaw` :type "Float (double-precision)") (`Pre Aim Off Set Pitch` :type "Float (double-precision)"))
  (locals (`Point A Loc` :type "Vector Structure") (`Point B Loc` :type "Vector Structure") (`Point C loc` :type "Vector Structure") (`Point E Loc` :type "Vector Structure") (`A Value` :type "Float (double-precision)") (`C Value` :type "Float (double-precision)") (AimOffSetYaw :type "Float (double-precision)") (`E Value` :type "Float (double-precision)") (AimOffSetPitch :type "Float (double-precision)") (`CameraMirror Loc` :type Boolean))
  (bind (_returnvalue_x _returnvalue_y _returnvalue_z) (`KismetMathLibrary.BreakVector` (- (`local.Point E Loc`) (`local.Point C loc`))))
  ;[1 1 1] Initialize Points
  (set `local.Point A Loc` `Point A`)
  (set `local.Point B Loc` `Point B`)
  (set `local.Point C loc` `Point C`)
  (set `local.Point E Loc` `Point E`)
  (set `local.CameraMirror Loc` `CameraMirror?`)
  ;[1 1 1] Aim Off Set Yaw Calculation
  (set `local.A Value` (`KismetMathLibrary.VSize` (- (`local.Point B Loc`) (`local.Point C loc`))))
  (set `local.C Value` (`KismetMathLibrary.VSize` (- (`local.Point C loc`) (`local.Point A Loc`))))
  (set `local.AimOffSetYaw` (`KismetMathLibrary.FClamp` (- 90.0 (`KismetMathLibrary.DegAsin` (/ (`local.A Value`) (`local.C Value`)))) 0.0 10.0))
  ;[1 1 1] Camera Mirror Condition
  (if (`local.CameraMirror Loc`)
    (set `local.AimOffSetYaw` (* (`local.AimOffSetYaw`) -1.0))
    (else
      (set `local.AimOffSetYaw` (`local.AimOffSetYaw`))))
  ;[1 1 1] Aim Off Set Pitch Calculation
  (set `local.E Value` (`KismetMathLibrary.VSize` (- (`local.Point E Loc`) (`local.Point C loc`))))
  (set `local.AimOffSetPitch` (`KismetMathLibrary.DegAsin` (/ (`local.E Value`) (`local.A Value`))))
  (if (< _returnvalue_z 0.0)
    (set `local.AimOffSetPitch` (`local.AimOffSetPitch`))
    (else
      (set `local.AimOffSetPitch` (* (`local.AimOffSetPitch`) -1.0))))
  (return (`local.AimOffSetYaw`) (`local.AimOffSetPitch`)))

(fn `AimOffSetPointsCalculation`
  (params (`Weapon Target Location` :type "Vector Structure"))
  (returns (`Point A` :type "Vector Structure") (`Point B` :type "Vector Structure") (`Point C` :type "Vector Structure") (`Point E` :type "Vector Structure"))
  (locals (`Point A Loc` :type "Vector Structure") (`Point B Loc` :type "Vector Structure") (`Point C Loc` :type "Vector Structure") (`Point E Loc` :type "Vector Structure") (`Point A Z Value` :type "Float (double-precision)"))
  (set `local.Point C Loc` `Weapon Target Location`)
  ;[1 1 1] Point A
  (set `local.Point A Loc` (`KismetMathLibrary.MakeVector` (.x (`self.Spring Arm World Location`)) (.y (`self.Spring Arm World Location`)) (+ (.z (`self.Spring Arm World Location`)) (.z (`self.Spring Arm Socet Offset`)))))
  ;[1 1 1] Point B
  (set `local.Point B Loc` (`KismetMathLibrary.MakeVector` (.x (+ (`local.Point A Loc`) (* (`KismetMathLibrary.GreaterGreater_VectorRotator` (`KismetMathLibrary.GetForwardVector` (`self.Character Actor Rotation`)) (struct :`Yaw` 90.0)) (.y (`self.Spring Arm Socet Offset`))))) (.y (+ (`local.Point A Loc`) (* (`KismetMathLibrary.GreaterGreater_VectorRotator` (`KismetMathLibrary.GetForwardVector` (`self.Character Actor Rotation`)) (struct :`Yaw` 90.0)) (.y (`self.Spring Arm Socet Offset`))))) (.z (+ (`local.Point A Loc`) (* (`KismetMathLibrary.GreaterGreater_VectorRotator` (`KismetMathLibrary.GetForwardVector` (`self.Character Actor Rotation`)) (struct :`Yaw` 90.0)) (.y (`self.Spring Arm Socet Offset`)))))))
  ;[1 1 1] Point E
  (set `local.Point E Loc` (`KismetMathLibrary.MakeVector` (.x (`local.Point C Loc`)) (.y (`local.Point C Loc`)) (.z (`local.Point B Loc`))))
  (return (`local.Point A Loc`) (`local.Point B Loc`) (`local.Point C Loc`) (`local.Point E Loc`)))

(fn `CreateWeaponTargetTrace`
  (params (Collision :type Boolean))
  (returns (WeaponTargetLocation :type "Vector Structure"))
  (locals (`Loc Collision` :type Boolean) (WithoutBlokcingObjectTypes :type "Array of EObjectTypeQuery Enum") (WithBlokcingObjectTypes :type "Array of EObjectTypeQuery Enum") (ObjectTypes :type "Array of EObjectTypeQuery Enum") (`Target Point` :type "Vector Structure" :default (0.0 0.0 0.0)))
  (bind _camera_world_location (`self.Camera World Location`))
  ;[1 1 1] Initialize Values
  (set `local.Loc Collision` Collision)
  (set `local.WithoutBlokcingObjectTypes` (`|MakeArray` "ObjectTypeQuery3" "ObjectTypeQuery1" "ObjectTypeQuery4" :!type "EObjectTypeQuery Enum"))
  (set `local.WithBlokcingObjectTypes` (`|MakeArray` "ObjectTypeQuery5" :!type "EObjectTypeQuery Enum"))
  ;[1 1 1] Collision Condition
  (if (`local.Loc Collision`)
    (set `local.ObjectTypes` (`local.WithBlokcingObjectTypes`))
    (else
      (set `local.ObjectTypes` (`local.WithoutBlokcingObjectTypes`))))
  (bind _outhit (`KismetSystemLibrary.LineTraceSingleForObjects` _camera_world_location (+ _camera_world_location (* (`KismetMathLibrary.GetForwardVector` (`self.Camera World Rotation`)) 2000.0)) (`local.ObjectTypes`) false (`|MakeArray` (`self.Character`) :!type "Actor Object Reference") "None" true (struct :`R` 1.0 :`B` 0.559379 :`A` 1.0) (struct :`G` 1.0 :`A` 1.0) 0.5))
  (bind (_bblockinghit _binitialoverlap _time _distance _location _impactpoint _normal _impactnormal _physmat _hitactor _hitcomponent _hitbonename _hititem _faceindex _tracestart _traceend) (`GameplayStatics.BreakHitResult` _outhit))
  (if _bblockinghit
    (set `local.Target Point` _location)
    (else
      (set `local.Target Point` _traceend)))
  (return (`local.Target Point`)))

(fn `WeaponDirectionFinalCalculation`
  (params (`Pre Weapon Yaw` :type "Float (double-precision)") (`Pre Weapon Pitch` :type "Float (double-precision)") (`Point E` :type "Vector Structure") (`Point C` :type "Vector Structure") (`Pre Aim Off Set Yaw` :type "Float (double-precision)") (`Pre Aim Off Set Pitch` :type "Float (double-precision)") (`Vertical Recoil Impact` :type "Float (double-precision)") (`Horizontal Recoil Impact` :type "Float (double-precision)"))
  (returns (`Weapon Direction` :type "Rotator Structure"))
  (locals (`Pre Weapon Yaw Loc` :type "Float (double-precision)") (`Pre Weapon Pitch Loc` :type "Float (double-precision)") (`Point E Loc` :type "Vector Structure") (`Point C Loc` :type "Vector Structure") (`Pre Aim Off Set Yaw Loc` :type "Float (double-precision)") (`Pre Aim Off Set Pitch Loc` :type "Float (double-precision)") (`Loc Weapon Direction Yaw` :type "Float (double-precision)") (`Loc Weapon Direction Pitch` :type "Float (double-precision)") (`Weapon Direction Loc` :type "Rotator Structure") (WeponDirVerRecCoeff :type "Float (double-precision)" :default 0.9) (WeponDirHorRecCoeff :type "Float (double-precision)" :default 0.3) (`Vertical Recoil Impact Loc` :type "Float (double-precision)") (`Horizontal Recoil Impact Loc` :type "Float (double-precision)"))
  ;[1 1 1] Initialize
  (set `local.Pre Weapon Yaw Loc` `Pre Weapon Yaw`)
  (set `local.Pre Weapon Pitch Loc` `Pre Weapon Pitch`)
  (set `local.Point E Loc` `Point E`)
  (set `local.Point C Loc` `Point C`)
  (set `local.Pre Aim Off Set Yaw Loc` `Pre Aim Off Set Yaw`)
  (set `local.Pre Aim Off Set Pitch Loc` `Pre Aim Off Set Pitch`)
  (set `local.Vertical Recoil Impact Loc` `Vertical Recoil Impact`)
  (set `local.Horizontal Recoil Impact Loc` `Horizontal Recoil Impact`)
  ;[1 1 1] Yaw Calculation
  (set `local.Loc Weapon Direction Yaw` (- (`local.Pre Aim Off Set Yaw Loc`) (`local.Pre Weapon Yaw Loc`)))
  ;[1 1 1] Pitch Calculation
  (if (< 0.0 (`local.Pre Weapon Pitch Loc`))
    (set `local.Loc Weapon Direction Pitch` (`KismetMathLibrary.Abs` (- (`KismetMathLibrary.Abs` (`local.Pre Aim Off Set Pitch Loc`)) (`KismetMathLibrary.Abs` (`local.Pre Weapon Pitch Loc`)))))
    (else
      (set `local.Loc Weapon Direction Pitch` (- (`KismetMathLibrary.Abs` (`local.Pre Aim Off Set Pitch Loc`)) (`KismetMathLibrary.Abs` (`local.Pre Weapon Pitch Loc`))))))
  ;[1 1 1] Final Calculation Weapon Direction & Support Recoil Impact
  (bind _output_get (set `local.Weapon Direction Loc` (`KismetMathLibrary.MakeRotator` 0.0 (+ (`local.Loc Weapon Direction Pitch`) (* (`local.Vertical Recoil Impact Loc`) (`local.WeponDirVerRecCoeff`))) (`KismetMathLibrary.FClamp` (+ 180.0 (`local.Loc Weapon Direction Yaw`) (* (`local.Horizontal Recoil Impact Loc`) (`local.WeponDirHorRecCoeff`))) 180.0 200.0))))
  (return _output_get))

(fn `WeaponDirectionPointCalculation`
  (params (`Weapon Target Point` :type "Vector Structure") (`Additional Point B` :type "Vector Structure") (`Camera Mirror` :type Boolean) (`Weapon Arrow Loc\\` :type "Vector Structure"))
  (returns (`Point A` :type "Vector Structure") (`Point B` :type "Vector Structure") (`Point C` :type "Vector Structure") (`Point E` :type "Vector Structure"))
  (locals (`Point A Loc` :type "Vector Structure") (`Point B Loc` :type "Vector Structure") (`Point C Loc` :type "Vector Structure") (`Point E Loc` :type "Vector Structure") (`Point P Loc` :type "Vector Structure") (`Value C` :type "Float (double-precision)") (`Value B` :type "Float (double-precision)") (`Value A` :type "Float (double-precision)") (`Value P` :type "Float (double-precision)") (`Value H` :type "Float (double-precision)") (`Additional Point B Loc` :type "Vector Structure") (`Camera Mirror Loc?` :type Boolean))
  ;[1 1 1] Initialize
  (set `local.Point C Loc` `Weapon Target Point`)
  (set `local.Additional Point B Loc` `Additional Point B`)
  (set `local.Camera Mirror Loc?` `Camera Mirror`)
  ;[1 1 1] Calculation Points
  (set `local.Point A Loc` `Weapon Arrow Loc\\`)
  (set `local.Point P Loc` (`KismetMathLibrary.MakeVector` (.x (`local.Additional Point B Loc`)) (.y (`local.Additional Point B Loc`)) (.z `Weapon Arrow Loc\\`)))
  (set `local.Point E Loc` (`KismetMathLibrary.MakeVector` (.x (`local.Point C Loc`)) (.y (`local.Point C Loc`)) (.z (`local.Point P Loc`))))
  ;[1 1 1] Calculation Values
  (set `local.Value C` (`KismetMathLibrary.VSize` (- (`local.Point E Loc`) (`local.Point A Loc`))))
  (set `local.Value B` (`KismetMathLibrary.VSize` (- (`local.Point A Loc`) (`local.Point P Loc`))))
  (set `local.Value A` (`KismetMathLibrary.VSize` (- (`local.Point E Loc`) (`local.Point P Loc`))))
  (set `local.Value P` (/ (+ (`local.Value C`) (`local.Value B`) (`local.Value A`)) 2.0))
  (set `local.Value H` (/ (* (`KismetMathLibrary.Sqrt` (* (`local.Value P`) (- (`local.Value P`) (`local.Value A`)) (- (`local.Value P`) (`local.Value B`)) (- (`local.Value P`) (`local.Value C`)))) 2.0) (`local.Value A`)))
  ;[1 1 1] Camera Mirror Logic
  (if (`local.Camera Mirror Loc?`)
    (set `local.Value H` (* -1.0 (`local.Value H`)))
    (else
      (set `local.Value H` (`local.Value H`))))
  ;[1 1 1] Point B Calculation
  (set `local.Point B Loc` (+ (`local.Point A Loc`) (* (`KismetMathLibrary.GreaterGreater_VectorRotator` (`KismetMathLibrary.GetForwardVector` (`self.Character Actor Rotation`)) (struct :`Yaw` 90.0)) (`local.Value H`))))
  (return (`local.Point A Loc`) (`local.Point B Loc`) (`local.Point C Loc`) (`local.Point E Loc`)))

(fn `WeaponDirectionPreCalculation`
  (params (`Point A` :type "Vector Structure") (`Point B` :type "Vector Structure") (`Point C` :type "Vector Structure") (`Point E` :type "Vector Structure"))
  (returns (`Pre Weapon Yaw` :type "Float (double-precision)") (`Pre Weapon Pitch` :type "Float (double-precision)"))
  (locals (`Point A Loc` :type "Vector Structure") (`Point B Loc` :type "Vector Structure") (`Point C Loc` :type "Vector Structure") (`Point E Loc` :type "Vector Structure") (`Value A` :type "Float (double-precision)") (`Value C` :type "Float (double-precision)") (`Value E` :type "Float (double-precision)") (Yaw :type "Float (double-precision)") (Pitch :type "Float (double-precision)"))
  (bind (_returnvalue_x _returnvalue_y _returnvalue_z) (`KismetMathLibrary.BreakVector` (- (`local.Point E Loc`) (`local.Point C Loc`))))
  ;[1 1 1] Initialize
  (set `local.Point A Loc` `Point A`)
  (set `local.Point B Loc` `Point B`)
  (set `local.Point C Loc` `Point C`)
  (set `local.Point E Loc` `Point E`)
  ;[1 1 1] Yaw Calculation
  (set `local.Value A` (`KismetMathLibrary.VSize` (- (`local.Point B Loc`) (`local.Point C Loc`))))
  (set `local.Value C` (`KismetMathLibrary.VSize` (- (`local.Point C Loc`) (`local.Point A Loc`))))
  (set `local.Yaw` (`KismetMathLibrary.FClamp` (- 90.0 (`KismetMathLibrary.DegAsin` (/ (`local.Value A`) (`local.Value C`)))) -20.0 20.0))
  ;[1 1 1] Pitch Calculation
  (set `local.Value E` (`KismetMathLibrary.VSize` (- (`local.Point E Loc`) (`local.Point C Loc`))))
  (set `local.Pitch` (`KismetMathLibrary.DegAsin` (/ (`local.Value E`) (`local.Value A`))))
  (if (< _returnvalue_z 0.0)
    (set `local.Pitch` (`local.Pitch`))
    (else
      (set `local.Pitch` (* (`local.Pitch`) -1.0))))
  (return (`local.Yaw`) (`local.Pitch`)))