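; Third-person shooter character that layers weapons, sniper scope and cover logic onto its parent class.
; BeginPlay spawns primary and secondary weapons on GunSocket and initializes the weapon system; a pickup dispatcher re-attaches and reinitializes them.
; A delayed-open Tick gate updates sprint rotation and velocity, plus authority-only front-space, cover and weapon-direction checks, the latter feeding replicated aim offsets.
; Scope events adjust camera FOV, and Enter opens a hard-coded server IP.
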(event `self.ReceiveBeginPlay`
  ;[1 1 1] Comment
  (`parent.ReceiveBeginPlay`)
  ;;[1 1 1] CHILD. BIND ON DISPATCHERS
  (`self.BindOnDispatchers`)
  ;;[1 1 1] Spawn Weapon
  (`self.TestSpawnWeapons`)
  (`KismetSystemLibrary.Delay` 0.1)
  (`self.MulticastInitializeCurrentWeaponInCharacter`)
  (`self.CommonInitializeWeaponSystem` (`self.Camera`) self null false false (`|MakeArray` "/Game/TPSCharacterSystem/Blueprints/Common/Misc/BP_WeaponRangeDoll.BP_WeaponRangeDoll_C" "/Game/TPSCharacterSystem/Blueprints/TPSCS/BP_TPSAICharacter.BP_TPSAICharacter_C" "BP_TPSCharacter_C" :!type "Object Class Reference"))
  (`self.InitializeWeaponInWeaponSystem`)
  ;;;[1 1 1] Comment
  (if (`self.SpawnWithOutWeapon?`)
    (set `self.WithOutWeapon?` true)
    (`self.SetActorHiddenInGame` (`self.PrimaryWeapon`) true)
    (`self.SetActorHiddenInGame` (`self.SecondaryWeapon`) true)
    (else
      (set `self.WithOutWeapon?` false)
      (`self.SetActorHiddenInGame` (`self.PrimaryWeapon`) false)
      (`self.SetActorHiddenInGame` (`self.SecondaryWeapon`) true)))
  (`KismetSystemLibrary.Delay` 0.5)
  (`self.OpenEventTick`))

(event `AttachWeapons`
  ;[1 1 1] SPAWN WEAPONS
  ;;[1 1 1] Attach
  (if (`self.PrimaryWeapon?`)
    (`/Engine/EditorBlueprintResources/StandardMacros.IsValid` (`self.PrimaryWeapon`)
      (:`Is Valid`
        (`self.K2_AttachToComponent` (`self.PrimaryWeapon`) (`self.Mesh`) "GunSocket" "SnapToTarget" "KeepRelative" "KeepRelative" true)))
    (else
      (`/Engine/EditorBlueprintResources/StandardMacros.IsValid` (`self.SecondaryWeapon`)
        (:`Is Valid`
          (`self.K2_AttachToComponent` (`self.SecondaryWeapon`) (`self.Mesh`) "GunSocket" "SnapToTarget" "KeepRelative" "KeepRelative" true))))))

(event `TestSpawnWeapons`
  ;[1 1 1] SPAWN WEAPONS
  (`/Engine/EditorBlueprintResources/StandardMacros.DoOnce` false
    (:`Completed`
      (`|ExecutionSequence`
        (:`then_0`
          ;;[1 1 1] Primary
          (bind _returnvalue (`|SpawnActorFromClass` (`self.PrimaryWeaponSpawnClass`) (`SceneComponent.GetRelativeTransform` (`self.Mesh`)) "AlwaysSpawn" "OverrideRootScale" null null))
          (bind _asbp_base_weapon (cast `/Game/TPSCharacterSystem/Blueprints/Common/WeaponsSystem/BaseWeapon/BP_BaseWeapon` _returnvalue))
          (bind _output_get (set `self.PrimaryWeapon` _asbp_base_weapon))
          (`/Engine/EditorBlueprintResources/StandardMacros.IsValid` _output_get
            (:`Is Valid`
              (`KismetSystemLibrary.Delay` 0.05)
              (`self.K2_AttachToComponent` (`self.PrimaryWeapon`) (`self.Mesh`) "GunSocket" "SnapToTarget" "KeepRelative" "KeepRelative" true)
              (`self.SetActorHiddenInGame` (`self.PrimaryWeapon`) false))))
        (:`then_1`
          ;;[1 1 1] Secondary
          (bind _returnvalue_2 (`|SpawnActorFromClass` (`self.SecondaryWeaponSpawnClass`) (`SceneComponent.GetRelativeTransform` (`self.Mesh`)) "AlwaysSpawn" "OverrideRootScale" null null))
          (bind _asbp_base_weapon_2 (cast `/Game/TPSCharacterSystem/Blueprints/Common/WeaponsSystem/BaseWeapon/BP_BaseWeapon` _returnvalue_2))
          (bind _output_get_2 (set `self.SecondaryWeapon` _asbp_base_weapon_2))
          (`/Engine/EditorBlueprintResources/StandardMacros.IsValid` _output_get_2
            (:`Is Valid`
              (`KismetSystemLibrary.Delay` 0.05)
              (`self.K2_AttachToComponent` (`self.SecondaryWeapon`) (`self.Mesh`) "GunSocket" "SnapToTarget" "KeepRelative" "KeepRelative" true)
              (`self.SetActorHiddenInGame` (`self.SecondaryWeapon`) true))))))))

(event `BindOnDispatchers`
  ;[1 1 1] Bind On Dicpatchers
  ;;[1 0.4027 0.05604] HandleOutPutPickuped
  (add `self.OutPutPickuped` (delegate `HandleOutPutPickuped`)))

(event `TPSSniperScoreOn`
  ;[1 1 1] SNIPER SCOPER
  ;;[1 1 1] SniperScoreOn
  ;;;[1 1 1] [common event]
  (`self.CommonSniperScopeOn` (`self.Mesh`) (`self.Camera`) (`self.Default Sniper Scoper FOV`)))

(event `HandleOutPutPickuped`
  ;[1 1 1] Bind On Dicpatchers
  ;;[1 0.4027 0.05604] HandleOutPutPickuped
  (`self.TellAllToChangeWeaponOn`)
  (`self.TellAllToPickUpWeapon`)
  (`KismetSystemLibrary.Delay` 0.5)
  (`self.ServerInitializeCurrentWeaponInCharacter`)
  (`self.AttachWeapons`)
  (`self.InitializeWeaponInWeaponSystem`))

(event `TPSSniperScoreOff`
  ;[1 1 1] SNIPER SCOPER
  ;;[1 1 1] SniperScoreOff
  ;;;[1 1 1] Get From TPS Controller Current FOV from camera component
  (bind _asbp_tpsplayer_controller (cast `/Game/TPSCharacterSystem/Blueprints/TPSCS/BP_TPSPlayerController` (`self.GetController`)))
  ;;;[1 1 1] [common event]
  (`self.CommonSniperScopeOff` (`self.Mesh`) (`self.Camera`) (`/Game/TPSCharacterSystem/Blueprints/TPSCS/Camera/BP_AdvancedTPSCamera.Current Field of View` (`/Game/TPSCharacterSystem/Blueprints/TPSCS/BP_TPSPlayerController.BP_AdvancedTPSCamera` _asbp_tpsplayer_controller))))

(event `self.ReceiveTick`
  (params (DeltaSeconds :type "Float (single-precision)"))
  ;[1 1 1] EVENT TICK
  (`parent.ReceiveTick` DeltaSeconds)
  (`/Engine/EditorBlueprintResources/StandardMacros.Gate` true :!label _label
    (:`Exit`
      (`|ExecutionSequence`
        (:`then_0`
          (`self.AllUpdateSprintMeshRoration` (`self.Current Yaw Mesh Rotation`))
          (`self.UpdateCharacterVelocity`))
        (:`then_1`
          (`/Engine/EditorBlueprintResources/ActorMacros.Switch Has Authority`
            (:`Authority`
              ;;[1 1 1] Update FrontChecker
              (`self.UpdateCheckingFrontSpace` 20.0 (20.0 10.0 20.0))
              ;;[1 1 1] Weapon Direction
              (`self.UpdateWeaponDirecton`)
              ;;[1 1 1] Locomotion Edged State
              (`self.UpdateMinizoomStateInLowCover`)
              (`self.UpdateSprintEdgesStates`)
              ;;[1 1 1] Cover Analizer
              (`self.UpdateCoverSystem`))))))))

(event `OpenEventTick`
  ;[1 1 1] EVENT TICK
  (goto _label :!via `Open`))

(event `TPSSniperScoreUpDown`
  ;[1 1 1] SNIPER SCOPER
  ;;[1 1 1] SniperScoreUpDown
  ;;;[1 1 1] [common event]
  (`self.SniperScopeUpDown` (`self.Camera`) (`self.TPS Default Sniper Scoper FOV`) (`self.TPS SniperScopeSecondZoomFOV`)))

(event `UpdateWeaponDirecton`
  (bind _springarm (`self.SpringArm`))
  (bind _camera (`self.Camera`))
  (bind _bp_weapondirection (`self.BP_WeaponDirection`))
  ;[1 1 1] WEAPON DIRECTION
  ;;[1 1 1] Main Logic
  ;;;[1 1 1] Init
  (if (`self.PrimaryWeapon?`)
    (`/Engine/EditorBlueprintResources/StandardMacros.IsValid` (`self.PrimaryWeapon`)
      (:`Is Valid`
        (set `self.Main Weapon Arrow Loc` (`SceneComponent.K2_GetComponentLocation` (`/Game/TPSCharacterSystem/Blueprints/Common/WeaponsSystem/BaseWeapon/BP_BaseWeapon.MainArrow` (`self.PrimaryWeapon`))))))
    (else
      (`/Engine/EditorBlueprintResources/StandardMacros.IsValid` (`self.SecondaryWeapon`)
        (:`Is Valid`
          (set `self.Main Weapon Arrow Loc` (`SceneComponent.K2_GetComponentLocation` (`/Game/TPSCharacterSystem/Blueprints/Common/WeaponsSystem/BaseWeapon/BP_BaseWeapon.MainArrow` (`self.SecondaryWeapon`))))))))
  ;;;[1 1 1] Trigger Main Event From Weapon Dir Component
  (`/Game/TPSCharacterSystem/Blueprints/TPSCS/WeaponDirection/BP_WeaponDirection.CalculationWeaponDirection` (`self.BP_WeaponDirection`) (`self.CameraMirror?`) (`self.FronSpaceCollisition?`) (`self.In MiniZoom ?`) (`self.Main Weapon Arrow Loc`) (`SceneComponent.K2_GetComponentLocation` _camera) (`SceneComponent.K2_GetComponentRotation` _camera) (`SceneComponent.K2_GetComponentLocation` _springarm) (`SpringArmComponent.SocketOffset` _springarm) (`self.K2_GetActorRotation`))
  ;;;[1 1 1] Update
  (`self.ServerUpdateCharacterAimOffSet` (`/Game/TPSCharacterSystem/Blueprints/TPSCS/WeaponDirection/BP_WeaponDirection.Aim Off Set Yaw` _bp_weapondirection) (`/Game/TPSCharacterSystem/Blueprints/TPSCS/WeaponDirection/BP_WeaponDirection.Aim Off Set Pitch` _bp_weapondirection) (`/Game/TPSCharacterSystem/Blueprints/TPSCS/WeaponDirection/BP_WeaponDirection.Main Arrow Rotation` _bp_weapondirection) true))

(event `Key|Enter`
  (params (Key :type "Key Structure"))
  (:`Pressed`
    (`GameplayStatics.OpenLevel` "172.27.127.102:7777")))

(fn `UserConstructionScript`
  (`parent.UserConstructionScript`))