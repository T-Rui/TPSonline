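; Player controller for the TPS character that drives its camera, sniper scope and death respawn.
; Character state updates run an edge-triggered decision tree (SpecialBranch DoOnce gates) that picks presets such as sprint, melee, crouch, mini-zoom or dead for BPAdvancedTPSCamera.
; Dispatchers toggle the scope on mini-zoom and reload, while inputs switch scope level and mirror the shoulder view.
; Death disables input, respawns through BP_DefaultGameMode after a delay, then reinitializes the controller.
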(event `self.ReceiveBeginPlay`
  ;[1 1 1] EVENT BEGIN PLAY
  (`parent.ReceiveBeginPlay` :!label _label)
  ;;[1 1 1] Initialize Components
  (bind _asbp_tpscharacter (cast `/Game/TPSCharacterSystem/Blueprints/TPSCS/BP_TPSCharacter` (`self.K2_GetPawn`)))
  (set `self.Controlled TPS Character` _asbp_tpscharacter)
  (set `self.Spring Arm` (`/Game/TPSCharacterSystem/Blueprints/TPSCS/BP_TPSCharacter.SpringArm` (`self.Controlled TPS Character`)))
  (set `self.Camera` (`/Game/TPSCharacterSystem/Blueprints/TPSCS/BP_TPSCharacter.Camera` (`self.Controlled TPS Character`)))
  (`self.InitializeToClientCamera`)
  (`self.BindOnDispathers`))

(event `RespawnInitializeController`
  ;[1 1 1] EVENT BEGIN PLAY
  ;;[1 1 1] RespawnInitializeController
  (goto _label))

(event `InitializeToClientCamera`
  ;[1 1 1] INITIALIZE CAMERA
  (`/Engine/EditorBlueprintResources/StandardMacros.IsValid` (`self.BP_AdvancedTPSCamera`)
    (:`Is Valid`
      (`/Engine/EditorBlueprintResources/StandardMacros.IsValid` (`self.Spring Arm`)
        (:`Is Valid`
          (`/Engine/EditorBlueprintResources/StandardMacros.IsValid` (`self.Camera`)
            (:`Is Valid`
              (`/Game/TPSCharacterSystem/Blueprints/TPSCS/Camera/BP_AdvancedTPSCamera.Set Start Camera Mode` (`self.BP_AdvancedTPSCamera`) (`self.Spring Arm`) (`self.Camera`) "FloorIdle" 65.0 -65.0))))))))

(event `self.ReceiveTick`
  (params (DeltaSeconds :type "Float (single-precision)"))
  ;[1 1 1] EVENT TICK
  (`parent.ReceiveTick` DeltaSeconds))

(event `BindOnDispathers`
  ;[1 1 1] BIND ON DISPATCHERS
  ;;[1 1 1] HandleCameraStateChanged
  (add `/Game/TPSCharacterSystem/Blueprints/TPSCS/Camera/BP_AdvancedTPSCamera.CameraStateChanged` (`self.BP_AdvancedTPSCamera`) (delegate `HandleCameraStateChanged`))
  ;;[1 0.4027 0.05604] HandleOutPutMiniZoomOff
  (add `/Game/TPSCharacterSystem/Blueprints/Common/BP_CommonCharacter.OutPutMiniZoomOff` (`self.Controlled TPS Character`) (delegate `HandleOutPutMiniZoomOff`))
  ;;[1 0.4027 0.05604] HandleOutPutReload
  (add `/Game/TPSCharacterSystem/Blueprints/Common/BP_CommonCharacter.OutPutReload` (`self.Controlled TPS Character`) (delegate `HandleOutPutReload`))
  ;;[1 0.4027 0.05604] HandleUpdateCharacterState
  (add `/Game/TPSCharacterSystem/Blueprints/Common/BP_CommonCharacter.OutPutUpdateCharacterState` (`self.Controlled TPS Character`) (delegate `HandleUpdateCharacterState`))
  ;;[1 0.4027 0.05604] HandleOutPutDead
  (add `/Game/TPSCharacterSystem/Blueprints/Common/BP_CommonCharacter.OutPutDead` (`self.Controlled TPS Character`) (delegate `HandleOutPutDead`)))

(event `HandleCameraStateChanged`
  (params (`Current Camera State` :type Name))
  ;[1 1 1] BIND ON DISPATCHERS
  ;;[1 1 1] HandleCameraStateChanged
  (if (or (== `Current Camera State` "FloorMiniZoom") (== `Current Camera State` "CrouchMiniZoom") (== `Current Camera State` "CrouchMiniZoomWalk"))
    (`/Game/TPSCharacterSystem/Blueprints/TPSCS/BP_TPSCharacter.TPSSniperScoreOn` (`self.Controlled TPS Character`))))

(event `HandleOutPutReload`
  ;[1 1 1] BIND ON DISPATCHERS
  ;;[1 0.4027 0.05604] HandleOutPutReload
  (`/Game/TPSCharacterSystem/Blueprints/TPSCS/BP_TPSCharacter.TPSSniperScoreOff` (`self.Controlled TPS Character`))
  (`KismetSystemLibrary.Delay` (`/Game/TPSCharacterSystem/Blueprints/Common/BP_CommonCharacter.Current Weapon Reload Time` (`self.Controlled TPS Character`)))
  (if (`self.MiniZoomHolding?`)
    (`/Game/TPSCharacterSystem/Blueprints/TPSCS/BP_TPSCharacter.TPSSniperScoreOn` (`self.Controlled TPS Character`))
    (else
      (`/Game/TPSCharacterSystem/Blueprints/Common/BP_CommonCharacter.TellServerToMiniZoomOff` (`self.Controlled TPS Character`)))))

(event `HandleUpdateCharacterState`
  (params (`In Minizoom?` :type Boolean) (`In Sprint?` :type Boolean) (`In Crouch?` :type Boolean) (`In Shooting ?` :type Boolean) (`Dead?` :type Boolean) (`In Melee?` :type Boolean) (`Move?` :type Boolean) (`In Climb Low Cover ?` :type Boolean) (`Jump Over Low Cover ?` :type Boolean) (`Is Falling?` :type Boolean) (`NearWall?` :type Boolean))
  ;[1 1 1] BIND ON DISPATCHERS
  ;;[1 0.4027 0.05604] HandleUpdateCharacterState
  ;;;[1 1 1] CAMERA CONTROLLER
  (`self.CameraController`))

(event `HandleOutPutMiniZoomOff`
  ;[1 1 1] BIND ON DISPATCHERS
  ;;[1 0.4027 0.05604] HandleOutPutMiniZoomOff
  (`/Game/TPSCharacterSystem/Blueprints/TPSCS/BP_TPSCharacter.TPSSniperScoreOff` (`self.Controlled TPS Character`)))

(event `HandleOutPutDead`
  ;[1 1 1] BIND ON DISPATCHERS
  ;;[1 0.4027 0.05604] HandleOutPutDead
  (`self.HandleDead`))

(event `InputAction|SniperScopeChange`
  (params (Key :type "Key Structure"))
  ;[1 1 1] SNIPER SCOPE INPUTS
  (:`Pressed`
    (`/Game/TPSCharacterSystem/Blueprints/TPSCS/BP_TPSCharacter.TPSSniperScoreUpDown` (`self.Controlled TPS Character`))))

(event `InputAction|CameraMirror`
  (params (Key :type "Key Structure"))
  ;[1 1 1] CAMERA MIRROR
  (:`Pressed`
    ;;[1 1 1] In Spire Score Condition
    (if (not (`/Game/TPSCharacterSystem/Blueprints/Common/BP_CommonCharacter.In Sniper Scope?` (`self.ControlledCommonCharacter`)))
      (if (`/Game/TPSCharacterSystem/Blueprints/TPSCS/BP_TPSCharacter.CameraMirror?` (`self.Controlled TPS Character`))
        (set `/Game/TPSCharacterSystem/Blueprints/TPSCS/BP_TPSCharacter.CameraMirror?` false (`self.Controlled TPS Character`))
        (else
          (set `/Game/TPSCharacterSystem/Blueprints/TPSCS/BP_TPSCharacter.CameraMirror?` true (`self.Controlled TPS Character`))))
      (`/Game/TPSCharacterSystem/Blueprints/TPSCS/Camera/BP_AdvancedTPSCamera.OpenGateChange` (`self.BP_AdvancedTPSCamera`))
      (`self.ChangeCameraState` (`/Game/TPSCharacterSystem/Blueprints/TPSCS/Camera/BP_AdvancedTPSCamera.Current Camera Mode` (`self.BP_AdvancedTPSCamera`))))))

(event `InputAction|SniperScopeDown`
  (params (Key :type "Key Structure"))
  ;[1 1 1] SNIPER SCOPE INPUTS
  (:`Pressed`
    (`/Game/TPSCharacterSystem/Blueprints/TPSCS/BP_TPSCharacter.TPSSniperScoreUpDown` (`self.Controlled TPS Character`))))

(event `InputAction|SniperScopeUp`
  (params (Key :type "Key Structure"))
  ;[1 1 1] SNIPER SCOPE INPUTS
  (:`Pressed`
    (`/Game/TPSCharacterSystem/Blueprints/TPSCS/BP_TPSCharacter.TPSSniperScoreUpDown` (`self.Controlled TPS Character`))))

(event `HandleDead`
  ;[1 1 1] RESPAWN
  ;;[1 1 1] Handle Respawn
  (`self.DisableInput` null)
  (`KismetSystemLibrary.Delay` 5.0)
  (`self.CharacterRespawn`)
  (`KismetSystemLibrary.Delay` 0.1)
  (`self.EnableInputEvent`)
  (`self.RespawnInitializeController`))

(event `EnableInputEvent`
  ;[1 1 1] RESPAWN
  ;;[1 1 1] Enable Input Event
  (`self.EnableInput` null)
  (`self.SetControlRotation` (`KismetMathLibrary.MakeRotator` (.roll (`self.GetControlRotation`)) 0.0 (.yaw (`self.GetControlRotation`)))))

(event `CharacterRespawn`
  ;[1 1 1] RESPAWN
  ;;[1 1 1] Main Respawn Logic
  (`/Engine/EditorBlueprintResources/ActorMacros.Switch Has Authority`
    (:`Authority`
      (`/Engine/EditorBlueprintResources/StandardMacros.IsValid` self
        (:`Is Valid`
          (bind _asbp_default_game_mode (cast `/Game/TPSCharacterSystem/Blueprints/TPSCS/BP_DefaultGameMode` (`GameplayStatics.GetGameMode`)))
          (`/Engine/EditorBlueprintResources/StandardMacros.IsValid` self
            (:`Is Valid`
              (`/Game/TPSCharacterSystem/Blueprints/TPSCS/BP_DefaultGameMode.CharacterRespawn` _asbp_default_game_mode self))))))))

(event `CameraController`
  ;[1 1 1] CameraController
  (`|ExecutionSequence`
    (:`then_0`
      (`self.SpecialBranch` (`self.Dead?`)
        (:`State On`
          ;[1 1 1] Dead State
          (`self.ChangeCameraState` "Dead"))))
    (:`then_1`
      (`self.SpecialBranch` (`self.In Sprint?`)
        (:`State On`
          ;[1 1 1] Sprint State
          (`self.ChangeCameraState` "FloorSprint"))
        (:`State Off`
          (`self.CheckStateMeleeSprintOff` :!label _label
            (:`MinizoomCrouchMove`
              ;[1 1 1] Crouch Minizoom Walk
              (`self.ChangeCameraState` "CrouchMiniZoomWalk" :!label _label_2))
            (:`MinizoomCrouch`
              ;[1 1 1] Crouch Minizoom State
              (`self.ChangeCameraState` "CrouchMiniZoom" :!label _label_3))
            (:`MinizoomFloorMove`
              ;[1 1 1] Floor Minizoom State
              (`self.ChangeCameraState` "FloorMiniZoom" :!label _label_4))
            (:`MinizzomFloorIdle`
              (goto _label_4))
            (:`CrouchMove`
              ;[1 1 1] Crouch Walk State
              (`self.ChangeCameraState` "CrouchWalk" :!label _label_5))
            (:`Crouch`
              ;[1 1 1] Crouch Idle State
              (`self.ChangeCameraState` "CrouchIdle" :!label _label_6))
            (:`FloorRun`
              ;[1 1 1] Floor Run state
              (`self.ChangeCameraState` "FloorRun" :!label _label_7))
            (:`FloorIdle`
              ;[1 1 1] Floor Idle State
              (`self.ChangeCameraState` "FloorIdle" :!label _label_8))))))
    (:`then_2`
      (`self.SpecialBranch` (`self.In Melee?`)
        (:`State On`
          ;[1 1 1] Melee State
          (`self.ChangeCameraState` "FloorMelee"))
        (:`State Off`
          (goto _label))))
    (:`then_3`
      (if (not (or (`self.Dead?`) (`self.In Sprint?`) (`self.In Melee?`)))
        (`|ExecutionSequence`
          (:`then_0`
            (`self.SpecialBranch` (`self.In Minizoom?`)
              (:`State On`
                (`self.CheckStateMinizoomOnOff`
                  (:`Crouch Move`
                    (goto _label_2))
                  (:`Crouch`
                    (goto _label_3))
                  (:`FloorMove`
                    (goto _label_4))
                  (:`FloorIdle`
                    (goto _label_4))))
              (:`State Off`
                (`self.CheckStateMinizoomOnOff`
                  (:`Crouch Move`
                    (goto _label_5))
                  (:`Crouch`
                    (goto _label_6))
                  (:`FloorMove`
                    (goto _label_7))
                  (:`FloorIdle`
                    (goto _label_8))))))
          (:`then_1`
            (`self.SpecialBranch` (`self.In Crouch?`)
              (:`State On`
                (`self.CheckStateCrouchOnOff`
                  (:`Minizoom Move`
                    (goto _label_2))
                  (:`Minizoom`
                    (goto _label_3))
                  (:`Move`
                    (goto _label_5))
                  (:`Idle`
                    (goto _label_6))))
              (:`State Off`
                (`self.CheckStateCrouchOnOff`
                  (:`Minizoom Move`
                    (goto _label_4))
                  (:`Minizoom`
                    (goto _label_4))
                  (:`Move`
                    (goto _label_7))
                  (:`Idle`
                    (goto _label_8))))))
          (:`then_2`
            (`self.SpecialBranch` (`self.Move?`)
              (:`State On`
                (`self.CheckStateMoveOnOff`
                  (:`CrouchMinizoom`
                    (goto _label_2))
                  (:`Crouch`
                    (goto _label_5))
                  (:`MinizoomFloor`
                    (goto _label_4))
                  (:`Floor`
                    (goto _label_7))))
              (:`State Off`
                (`self.CheckStateMoveOnOff`
                  (:`CrouchMinizoom`
                    (goto _label_3))
                  (:`Crouch`
                    (goto _label_6))
                  (:`MinizoomFloor`
                    (goto _label_4))
                  (:`Floor`
                    (goto _label_8)))))))))))

(fn `ChangeCameraState`
  (params (`Input Camera Preset` :type Name))
  (`/Game/TPSCharacterSystem/Blueprints/TPSCS/Camera/BP_AdvancedTPSCamera.OpenGateChange` (`self.BP_AdvancedTPSCamera`))
  (`/Game/TPSCharacterSystem/Blueprints/TPSCS/Camera/BP_AdvancedTPSCamera.Change Camera Mode` (`self.BP_AdvancedTPSCamera`) (`self.Spring Arm`) (`self.Camera`) `Input Camera Preset` (`/Game/TPSCharacterSystem/Blueprints/TPSCS/BP_TPSCharacter.CameraMirror?` (`self.Controlled TPS Character`))))

(fn `UserConstructionScript`
  (`parent.UserConstructionScript`))